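; Player controller for a turn-based tactical game, turning Enhanced Input into commands for units and turns.
; BeginPlay adds the shared mapping context; input events call functions for four actions, next unit, end turn and declining reactions.
; Move inputs impart velocity along fixed 2D axes, with a zero-degree rotation applied.
; Tick adds mouse X delta to control yaw and teleport-rotates the current unit from that rotation plus the delta again.
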(event `self.ReceiveBeginPlay`
  (`EnhancedInputSubsystemInterface.AddMappingContext` (subsystem `EnhancedInputLocalPlayerSubsystem`) "/Game/Input/IMC_Shared.IMC_Shared" 0 (struct)))

(event `EnhancedInput|/Game/Input/IA_MoveUp`
  (params (ActionValue :type Boolean) (ElapsedSeconds :type "Float (double-precision)") (TriggeredSeconds :type "Float (double-precision)") (InputAction :type "InputAction Object Reference" :default "/Game/Input/IA_MoveUp.IA_MoveUp"))
  ; movement
  (:`Triggered`
    (`self.ImpartVelocity` (`KismetMathLibrary.GetRotated2D` (1.0 0.0)))))

(event `EnhancedInput|/Game/Input/IA_Action1`
  (params (ActionValue :type Boolean) (ElapsedSeconds :type "Float (double-precision)") (TriggeredSeconds :type "Float (double-precision)") (InputAction :type "InputAction Object Reference" :default "/Game/Input/IA_Action1.IA_Action1"))
  ; actions
  (:`Triggered`
    (`self.Action1`)))

(event `EnhancedInput|/Game/Input/IA_Action2`
  (params (ActionValue :type Boolean) (ElapsedSeconds :type "Float (double-precision)") (TriggeredSeconds :type "Float (double-precision)") (InputAction :type "InputAction Object Reference" :default "/Game/Input/IA_Action2.IA_Action2"))
  ; actions
  (:`Triggered`
    (`self.Action2`)))

(event `EnhancedInput|/Game/Input/IA_EndTurn`
  (params (ActionValue :type Boolean) (ElapsedSeconds :type "Float (double-precision)") (TriggeredSeconds :type "Float (double-precision)") (InputAction :type "InputAction Object Reference" :default "/Game/Input/IA_EndTurn.IA_EndTurn"))
  ; turn management
  (:`Triggered`
    (`self.EndTurn`)))

(event `EnhancedInput|/Game/Input/IA_MoveDown`
  (params (ActionValue :type Boolean) (ElapsedSeconds :type "Float (double-precision)") (TriggeredSeconds :type "Float (double-precision)") (InputAction :type "InputAction Object Reference" :default "/Game/Input/IA_MoveDown.IA_MoveDown"))
  ; movement
  (:`Triggered`
    (`self.ImpartVelocity` (`KismetMathLibrary.GetRotated2D` (-1.0 0.0)))))

(event `EnhancedInput|/Game/Input/IA_Action3`
  (params (ActionValue :type Boolean) (ElapsedSeconds :type "Float (double-precision)") (TriggeredSeconds :type "Float (double-precision)") (InputAction :type "InputAction Object Reference" :default "/Game/Input/IA_Action3.IA_Action3"))
  ; actions
  (:`Triggered`
    (`self.Action3`)))

(event `EnhancedInput|/Game/Input/IA_Next`
  (params (ActionValue :type Boolean) (ElapsedSeconds :type "Float (double-precision)") (TriggeredSeconds :type "Float (double-precision)") (InputAction :type "InputAction Object Reference" :default "/Game/Input/IA_Next.IA_Next"))
  ; turn management
  (:`Triggered`
    (`self.NextUnit`)))

(event `EnhancedInput|/Game/Input/IA_MoveLeft`
  (params (ActionValue :type Boolean) (ElapsedSeconds :type "Float (double-precision)") (TriggeredSeconds :type "Float (double-precision)") (InputAction :type "InputAction Object Reference" :default "/Game/Input/IA_MoveLeft.IA_MoveLeft"))
  ; movement
  (:`Triggered`
    (`self.ImpartVelocity` (`KismetMathLibrary.GetRotated2D` (0.0 -1.0)))))

(event `EnhancedInput|/Game/Input/IA_Action4`
  (params (ActionValue :type Boolean) (ElapsedSeconds :type "Float (double-precision)") (TriggeredSeconds :type "Float (double-precision)") (InputAction :type "InputAction Object Reference" :default "/Game/Input/IA_Action4.IA_Action4"))
  ; actions
  (:`Triggered`
    (`self.Action4`)))

(event `EnhancedInput|/Game/Input/IA_DeclineReaction`
  (params (ActionValue :type Boolean) (ElapsedSeconds :type "Float (double-precision)") (TriggeredSeconds :type "Float (double-precision)") (InputAction :type "InputAction Object Reference" :default "/Game/Input/IA_DeclineReaction.IA_DeclineReaction"))
  ; turn management
  (:`Triggered`
    (`self.DeclineReaction`)))

(event `EnhancedInput|/Game/Input/IA_MoveRight`
  (params (ActionValue :type Boolean) (ElapsedSeconds :type "Float (double-precision)") (TriggeredSeconds :type "Float (double-precision)") (InputAction :type "InputAction Object Reference" :default "/Game/Input/IA_MoveRight.IA_MoveRight"))
  ; movement
  (:`Triggered`
    (`self.ImpartVelocity` (`KismetMathLibrary.GetRotated2D` (0.0 1.0)))))

(event `self.ReceiveTick`
  (params (DeltaSeconds :type "Float (single-precision)"))
  (bind _returnvalue (`KismetMathLibrary.MakeRotator` (.roll (`self.GetControlRotation`)) (.pitch (`self.GetControlRotation`)) (+ (.yaw (`self.GetControlRotation`)) (`self.GetInputMouseDelta`))))
  ; mouse camera
  (`self.SetControlRotation` _returnvalue)
  (`self.K2_SetActorRotation` (`self.GetCurrentUnit`) _returnvalue true))

(fn `UserConstructionScript`)